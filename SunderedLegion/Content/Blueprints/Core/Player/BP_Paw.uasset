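; BP_Paw is a player camera pawn with planar movement, stepped yaw rotation and spring arm zoom.
; Forward and right axes shift a desired location along the actor's own vectors, rotation presses step a desired yaw, and the zoom axis adjusts a clamped arm length.
; Tick eases location, rotation and arm length toward those targets with separate interpolation speeds, moving without sweep.
; Input increments are not scaled by delta time.
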(event `self.ReceiveBeginPlay`
  (set `self.LocationDesired` (`self.K2_GetActorLocation`))
  (set `self.ZoomDesired` (`SpringArmComponent.TargetArmLength` (`self.SpringArm`)))
  (set `self.RotationDesired` (`self.K2_GetActorRotation`)))

(event `self.ReceiveTick`
  (params (DeltaSeconds :type "Float (single-precision)"))
  (bind _springarm (`self.SpringArm`))
  (set `SpringArmComponent.TargetArmLength` (`KismetMathLibrary.FInterpTo` (`SpringArmComponent.TargetArmLength` _springarm) (`self.ZoomDesired`) DeltaSeconds (`self.ZoomInturp`)) _springarm)
  (`self.K2_SetActorLocation` (`KismetMathLibrary.VInterpTo` (`self.K2_GetActorLocation`) (`self.LocationDesired`) DeltaSeconds (`self.LocationInturp`)))
  (`self.K2_SetActorRotation` (`KismetMathLibrary.RInterpTo` (`self.K2_GetActorRotation`) (`self.RotationDesired`) DeltaSeconds (`self.RotationInturp`))))

(event `InputAxis|InputAxis_Zoom`
  (params (AxisValue :type "Float (single-precision)"))
  (set `self.ZoomDesired` (`KismetMathLibrary.FClamp` (+ (* AxisValue (`self.ZoomSpeed`)) (`self.ZoomDesired`)) (`self.ZoomMin`) (`self.ZoomMax`))))

(event `InputAxis|InputAxis_Forward`
  (params (AxisValue :type "Float (single-precision)"))
  (set `self.LocationDesired` (+ (`self.LocationDesired`) (* (* AxisValue (`self.LocationSpeed`)) (`self.GetActorForwardVector`)))))

(event `InputAxis|InputAxis_Right`
  (params (AxisValue :type "Float (single-precision)"))
  (set `self.LocationDesired` (+ (`self.LocationDesired`) (* (* AxisValue (`self.LocationSpeed`)) (`self.GetActorRightVector`)))))

(event `InputAction|InputAction_RotationLeft`
  (params (Key :type "Key Structure"))
  (:`Pressed`
    (set `self.RotationDesired` (`KismetMathLibrary.ComposeRotators` (`self.RotationDesired`) (`KismetMathLibrary.MakeRotator` 0.0 0.0 (`self.RotationSpeed`))))))

(event `InputAction|InputAction_RotationRight`
  (params (Key :type "Key Structure"))
  (:`Pressed`
    (set `self.RotationDesired` (`KismetMathLibrary.ComposeRotators` (`self.RotationDesired`) (`KismetMathLibrary.MakeRotator` 0.0 0.0 (- 0.0 (`self.RotationSpeed`)))))))

(fn `UserConstructionScript`)